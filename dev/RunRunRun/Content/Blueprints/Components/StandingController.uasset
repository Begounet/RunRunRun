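; StandingController is a component that controls the eye height of its owner by moving the owner's Camera component vertically.
; On BeginPlay it finds the camera, printing an error if none exists, and derives a ground offset from the Character's capsule half height.
; SetMaxHeight caps the height at no more than CharacterHeight and RestoreHeight lifts the cap, both immediately updating the camera's relative Z.
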(event EventBeginPlay
  (|CallParentFunction)
  (Init|Initialize))

(fn SetMaxHeight
  (params (Height :type Float%20%28single-precision%29))
  (Variables|Default|SetCurrentMaxHeight Height)
  (CallFunction|UpdateHeighttoCurrentMax))

(fn RestoreHeight
  (Init|ResetCurrentMaxHeight)
  (CallFunction|UpdateHeighttoCurrentMax))

(fn Initialize
  (bind _output_get (Variables|Default|SetOwnerCameraComponent (Actor|GetComponentbyClass (Components|GetOwner) "/Script/Engine.CameraComponent")))
  (Utilities|IsValid _output_get
    (:Is%20Valid
      (Init|InitializeGroundOffset)
      (Init|ResetCurrentMaxHeight))
    (:Is%20Not%20Valid
      (Development|PrintString "StandingController require a Camera component on its owner to work"))))

(fn UpdateHeighttoCurrentMax
  (bind _ownercameracomponent (Variables|Default|GetOwnerCameraComponent))
  (bind _relativelocation (Variables|/Script/Engine.SceneComponent|GetRelativeLocation _ownercameracomponent))
  (Transformation|SetRelativeLocation (Variables|Default|GetOwnerCameraComponent) (Math|Vector|MakeVector (.x _relativelocation) (.y _relativelocation) (- (CallFunction|GetMaxHeight) (Variables|Default|GetGroundOffset))) false false))

(fn GetMaxHeight
  (return (Math|Float|Min(Float) (Variables|Default|GetCharacterHeight) (Variables|Default|GetCurrentMaxHeight))))

(fn InitializeGroundOffset
  (bind _ascharacter (Utilities|Casting|CastToCharacter (Components|GetOwner)))
  (bind _result (Math|Float|NegateFloat (Components|Capsule|GetScaledCapsuleHalfHeight (Variables|/Script/Engine.Character|GetCapsuleComponent _ascharacter)))
    (:%20%20
      (Variables|Default|SetGroundOffset _result))))

(fn ResetCurrentMaxHeight
  (Variables|Default|SetCurrentMaxHeight (Variables|Default|GetCharacterHeight)))