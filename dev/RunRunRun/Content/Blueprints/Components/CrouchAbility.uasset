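; CrouchAbility is a component that tracks crouch state for its owner and is only partly implemented.
; StartCrouch and StopCrouch toggle IsCrouched, guarded against repeat calls, and call DecreaseHeight and RestoreHeight, which are both empty.
; On crouch start, ShouldSlide compares the owner's velocity magnitude against MinimumSpeedForSliding, but the slide branch does nothing yet.
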(event Custom|Start%20Crouch
  (if (not (Variables|Default|GetIsCrouched))
    (Variables|Default|SetIsCrouched true)
    (CallFunction|DecreaseHeight)
    (if (CallFunction|ShouldSlide)
      _)))

(event Custom|Stop%20Crouch
  (if (Variables|Default|GetIsCrouched)
    (Variables|Default|SetIsCrouched false)
    (CallFunction|RestoreHeight)))

(fn ShouldSlide
  (return (>= (Math|Vector|VectorLength (CallFunction|GetOwnerVelocity)) (Variables|Default|GetMinimumSpeedForSliding))))

(fn GetOwnerVelocity
  (return (Transformation|GetVelocity (Components|GetOwner))))

(fn DecreaseHeight)

(fn RestoreHeight)