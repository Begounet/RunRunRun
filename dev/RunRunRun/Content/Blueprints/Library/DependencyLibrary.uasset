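; Blueprint function library that validates component dependencies between actors and their components.
; Get functions look up a component by class, either on a given actor or on a component's owner, and return it.
; When the lookup fails, they print an on-screen dependency error naming the objects and missing class.
; Check variants run the same lookup purely for that warning, without returning the component.
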(fn CheckOwnerComponentDependency
  (params (SelfComponent :type Actor%20Component%20Object%20Reference) (ComponentClass :type Actor%20Component%20Class%20Reference))
  (CallFunction|GetOwnerComponentDependency SelfComponent ComponentClass))

(fn GetOwnerComponentDependency
  (params (SelfComponent :type Actor%20Component%20Object%20Reference) (ComponentClass :type Actor%20Component%20Class%20Reference))
  (bind _output_get (LocalVariables|SetComponent (Actor|GetComponentbyClass (Components|GetOwner SelfComponent) ComponentClass)))
  (Utilities|IsValid _output_get
    (:Is%20Valid
      _)
    (:Is%20Not%20Valid
      (Print|PrintOwnerComponentMissingDependency SelfComponent ComponentClass)))
  (return (LocalVariables|GetComponent)))

(fn PrintOwnerComponentMissingDependency
  (params (ActorComponent :type Actor%20Component%20Object%20Reference) (Class :type Actor%20Component%20Class%20Reference))
  (Development|PrintString 0 (Utilities|String|Append "Dependency error : " (Utilities|GetDisplayName ActorComponent) " couldn't get a component of class '" (Utilities|GetClassDisplayName Class) "' from its owner '" (Utilities|GetDisplayName (Components|GetOwner ActorComponent)) "'") true true "(R=1.000000,G=0.000000,B=0.000000,A=1.000000)" 5.0))

(fn GetComponentDependency
  (params (Actor :type Actor%20Object%20Reference) (ComponentClass :type Actor%20Component%20Class%20Reference))
  (bind _output_get (LocalVariables|SetComponent (Actor|GetComponentbyClass Actor ComponentClass)))
  (Utilities|IsValid _output_get
    (:Is%20Valid
      _)
    (:Is%20Not%20Valid
      (Print|PrintComponentMissingDependency Actor ComponentClass)))
  (return (LocalVariables|GetComponent)))

(fn CheckComponentDependency
  (params (Actor :type Actor%20Object%20Reference) (ComponentClass :type Actor%20Component%20Class%20Reference))
  (CallFunction|GetComponentDependency Actor ComponentClass))

(fn PrintComponentMissingDependency
  (params (Actor :type Actor%20Object%20Reference) (Component :type Actor%20Component%20Class%20Reference))
  (Development|PrintString 0 (Utilities|String|Append "Dependency error : " (Utilities|GetDisplayName Actor) "don't have a component of class '" (Utilities|GetClassDisplayName Component) "'") true true "(R=1.000000,G=0.000000,B=0.000000,A=1.000000)" 5.0))